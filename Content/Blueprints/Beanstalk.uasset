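; Beanstalk segment actor for a climbing game, carrying left, middle and right knots and exposing an attach point transform.
; SpawnKnots reads a three-character code (O, X or Q per slot) and adds child actor knots at slightly randomized spawn offsets.
; GetKnotVector returns a knot's world location by position index.
; When ClimbCharacter leaves its collision, it has ClimbGameMode add a new stalk and records it in the game mode's arrays.
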(event OnComponentEndOverlap(PlayerColission)
  (params (OtherActor :type Actor%20Object%20Reference) (OtherComp :type Primitive%20Component%20Object%20Reference) (OtherBodyIndex :type Integer))
  (Utilities|Casting|CastToClimbCharacter OtherActor)
  (bind _asclimb_game_mode (Utilities|Casting|CastToClimbGameMode (Game|GetGameMode)))
  (bind (_stalkpart _stalkreference _stalkindex) (Default|AddNewStalk _asclimb_game_mode))
  (Utilities|Array|Add (Variables|/Game/Blueprints/ClimbGameMode.ClimbGameMode_C|GetBeanstalk _asclimb_game_mode) _stalkpart)
  (Utilities|Array|Add (Variables|/Game/Blueprints/ClimbGameMode.ClimbGameMode_C|GetBeanStalkParts _asclimb_game_mode) _stalkreference)
  (Utilities|Array|Add (Variables|/Game/Blueprints/ClimbGameMode.ClimbGameMode_C|GetBeanstalkIndex _asclimb_game_mode) _stalkindex))

(event EventBeginPlay)

(event EventActorBeginOverlap
  (params (OtherActor :type Actor%20Object%20Reference)))

(event EventTick
  (params (DeltaSeconds :type Float%20%28single-precision%29)))

(fn ConstructionScript)

(fn GetAttachPoint
  (return (Transformation|GetWorldTransform (Variables|Default|GetAttachPoint))))

(fn SpawnKnots
  (params (NewBeanstalk :type String))
  (bind _returnvalue (Utilities|String|GetCharacterArrayfromString NewBeanstalk))
  (bind (_leftknottransform _middleknottransform _rightknottransform) (CallFunction|RandomizeKnotTransform))
  (switch name (Utilities|String|StringToName (Utilities|Array|Get(acopy) _returnvalue))
    (:Default
      _)
    (:O
      (bind _returnvalue_2 (AddComponent|AddChildActorComponent false _leftknottransform))
      (Variables|Default|SetLeftKnotReference _returnvalue_2))
    (:X
      (bind _returnvalue_3 (AddComponent|AddChildActorComponent false _leftknottransform))
      (Variables|Default|SetLeftKnotReference _returnvalue_3))
    (:Q
      (bind _returnvalue_4 (AddComponent|AddChildActorComponent false _leftknottransform))
      (Variables|Default|SetLeftKnotReference _returnvalue_4)))
  (switch name (Utilities|String|StringToName (Utilities|Array|Get(acopy) _returnvalue 1))
    (:Default
      _)
    (:O
      (bind _returnvalue_5 (AddComponent|AddChildActorComponent false _middleknottransform))
      (Variables|Default|SetMiddleKnotReference _returnvalue_5))
    (:X
      (bind _returnvalue_6 (AddComponent|AddChildActorComponent false _middleknottransform))
      (Variables|Default|SetMiddleKnotReference _returnvalue_6))
    (:Q
      (bind _returnvalue_7 (AddComponent|AddChildActorComponent false _middleknottransform))
      (Variables|Default|SetMiddleKnotReference _returnvalue_7)))
  (switch name (Utilities|String|StringToName (Utilities|Array|Get(acopy) _returnvalue 2))
    (:O
      (bind _returnvalue_8 (AddComponent|AddChildActorComponent false _rightknottransform))
      (Variables|Default|SetRightKnotReference _returnvalue_8))
    (:X
      (bind _returnvalue_9 (AddComponent|AddChildActorComponent false _rightknottransform))
      (Variables|Default|SetRightKnotReference _returnvalue_9))
    (:Q
      (bind _returnvalue_10 (AddComponent|AddChildActorComponent false _rightknottransform))
      (Variables|Default|SetRightKnotReference _returnvalue_10))))

(fn RandomizeKnotTransform
  (bind _returnvalue (Transformation|GetRelativeTransform (Variables|Default|GetKnotSpawnLeft)))
  (bind _returnvalue_2 (Transformation|GetRelativeTransform (Variables|Default|GetKnotSpawnMiddle)))
  (bind _returnvalue_3 (Transformation|GetRelativeTransform (Variables|Default|GetKnotSpawnRight)))
  (bind _uniquetransform (CallFunction|RandomizeTransform _returnvalue))
  (bind _uniquetransform_2 (CallFunction|RandomizeTransform _returnvalue_2))
  (bind _uniquetransform_3 (CallFunction|RandomizeTransform _returnvalue_3))
  (return _uniquetransform _uniquetransform_2 _uniquetransform_3))

(fn RandomizeTransform
  (params (StandardTransform :type Transform))
  (bind (_location _rotation _scale) (Math|Transform|BreakTransform StandardTransform))
  (bind (_x _y _z) (Math|Vector|BreakVector _location))
  (return (Math|Transform|MakeTransform (Math|Vector|MakeVector _x (+ _y (Math|Random|RandomFloatinRange -1e+01 1e+01)) (+ _z (Math|Random|RandomFloatinRange -15.0 15.0))) _rotation _scale)))

(fn GetKnotVector
  (params (Position :type Integer :default 0))
  (switch int Position
    (:Default
      _)
    (:0
      (LocalVariables|SetKnotVectorBuffer (Transformation|GetWorldLocation (Variables|Default|GetLeftKnotReference))))
    (:1
      (LocalVariables|SetKnotVectorBuffer (Transformation|GetWorldLocation (Variables|Default|GetMiddleKnotReference))))
    (:2
      (LocalVariables|SetKnotVectorBuffer (Transformation|GetWorldLocation (Variables|Default|GetRightKnotReference)))))
  (return (LocalVariables|GetKnotVectorBuffer)))